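; Game mode for MarsMarine that runs endless, escalating waves of enemies.
; Each wave scales its spawn count by a difficulty multiplier, then a looping timer spawns BP_Enemy_01 at random TargetPoints until the count runs out.
; Spawned enemies are tracked in an array that RegisterEnemyDeath trims.
; When no enemies or pending spawns remain, the next wave starts after a short delay.
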(event Custom|Spawn%20Wave
  (Enemy|SpawnEnemy))

(event Custom|End%20Wave
  (Utilities|FlowControl|Delay 2.0)
  (Wave|SetupWave))

(event EventBeginPlay
  (Utilities|FlowControl|Delay 2.0)
  (Wave|SetupWave))

(fn ConstructionScript)

(fn SpawnEnemy
  (bind _random_point (Enemy|GetRandonPoint))
  (Utilities|IsValid _random_point
    (:Is%20Valid
      (bind _returnvalue (Game|SpawnActorfromClass "/Game/Blueprints/AI/BP_Enemy_01.BP_Enemy_01_C" (Transformation|GetActorTransform _random_point) "Undefined" 0 0))
      (Utilities|IsValid _returnvalue
        (:Is%20Valid
          (Utilities|Array|Add (Variables|Enemy|GetEnemies) _returnvalue)
          (bind _result (Math|Integer|DecrementInt (Variables|Enemy|GetEnemy%20Spawns%20Remaining%20))
            (:%20%20
              (if (== _result 0)
                (Utilities|Time|ClearTimerbyFunctionName 0 "Spawn Wave")))))))))

(fn GetRandonPoint
  (bind _outactors (Actor|GetAllActorsOfClass "/Script/Engine.TargetPoint"))
  (return (Utilities|Array|Get(acopy) _outactors (Math|Random|RandomIntegerinRange 0 (Utilities|Array|LastIndex _outactors)))))

(fn RegisterEnemyDeath
  (params (Enemy :type BP%20Enemy%2001%20Object%20Reference%20%28by%20ref%29))
  (Utilities|Array|RemoveItem (Variables|Enemy|GetEnemies) Enemy)
  (if (Wave|IsWaveComplete)
    (CallFunction|EndWave)))

(fn IsWaveComplete
  (return (and (== (Utilities|Array|Length (Variables|Enemy|GetEnemies)) 0) (== (Variables|Enemy|GetEnemy%20Spawns%20Remaining%20) 0))))

(fn SetupWave
  (Math|Integer|IncrementInt (Variables|Wave|GetWave%20Counter)
    (:%20%20
      (Wave|IncreaseWaveDifficulty)
      (Utilities|Time|SetTimerbyFunctionName 0 "Spawn Wave" (Variables|Wave|GetSpawn%20Frequency) true))))

(fn GetNextWaveDifficulty
  (return (Math|Float|Round (* (Variables|Wave|GetWave%20Difficulty) (Variables|Wave|GetDifficulty%20Multiplier)))))

(fn IncreaseWaveDifficulty
  (bind _output_get (Variables|Wave|SetWave%20Difficulty (Wave|GetNextWaveDifficulty)))
  (Variables|Enemy|SetEnemy%20Spawns%20Remaining%20 _output_get))