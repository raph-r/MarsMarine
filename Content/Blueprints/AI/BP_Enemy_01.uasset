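; BP_Enemy_01 is a melee enemy that chases and attacks the player in what appears to be the Mars Marine game.
; A looping AIMoveTo drives the chase, while Tick halts movement and plays an attack montage within range, resuming on completion.
; DamagePlayer applies damage but is not called within this Blueprint.
; At zero health it disables collision, credits the marine's kill, notifies the game mode and is destroyed after a delay.
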(event EventBeginPlay
  (Variables|Default|SetHealth (Variables|Default|GetMax%20Health))
  ;[1 1 1] Charge Player
  (if (CallFunction|IsAlive) :!label _label
    (AI|AIMoveTo self "0, 0, 0" (Game|GetPlayerCharacter 0) 5.0 false
      (:OnSuccess
        _)
      (:OnFail
        _))
    (Utilities|FlowControl|Delay 0.2)
    (goto _label)))

(event Game|Damage|EventAnyDamage
  (params (Damage :type Float%20%28single-precision%29) (DamageType :type Damage%20Type%20Object%20Reference) (InstigatedBy :type Controller%20Object%20Reference) (DamageCauser :type Actor%20Object%20Reference))
  ;[1 1 1] Take Damage
  (if (CallFunction|IsAlive)
    (CallFunction|DecreaseHealth Damage)
    (if (== (Variables|Default|GetHealth) 0.0)
      (CallFunction|KillAI)
      (Utilities|FlowControl|Delay 3.0)
      (Actor|DestroyActor))))

(event EventTick
  (params (DeltaSeconds :type Float%20%28single-precision%29))
  ;[1 1 1] Attack Player
  (if (CallFunction|CanAttack)
    (CallFunction|DeactiveAIMovement)
    (Animation|Montage|PlayMontage (Variables|Character|GetMesh) "/Game/Characters/Enemy_Great_Spider/Animations/MeleeAttackMontage_01.MeleeAttackMontage_01"
      (:OnCompleted
        (CallFunction|ActiveAIMovement)))))

(fn ConstructionScript)

(fn IsWithinAttackRange
  (return (<= (Transformation|GetDistanceTo (Game|GetPlayerCharacter 0)) (Variables|Default|GetAttack%20Range))))

(fn IsAttacking
  (return (Animation|Montage|MontageIsPlaying (Components|SkeletalMesh|GetAnimInstance (Variables|Character|GetMesh)) "/Game/Characters/Enemy_Great_Spider/Animations/MeleeAttackMontage_01.MeleeAttackMontage_01")))

(fn DeactiveAIMovement
  (bind _charactermovement (Variables|Character|GetCharacterMovement))
  (Components|Movement|StopMovementImmediately _charactermovement)
  (Components|Activation|Deactivate _charactermovement))

(fn ActiveAIMovement
  (Components|Activation|Activate (Variables|Character|GetCharacterMovement) false))

(fn DamagePlayer
  (if (CallFunction|IsAlive)
    (Game|Damage|ApplyDamage (Game|GetPlayerCharacter 0) (Variables|Default|GetDamage) 0 0)))

(fn DecreaseHealth
  (params (Damage :type Float%20%28single-precision%29))
  (Variables|Default|SetHealth (Math|Float|Clamp(Float) (- (Variables|Default|GetHealth) Damage) 0.0 (Variables|Default|GetMax%20Health))))

(fn KillAI
  (Variables|Default|SetIs%20Dead true)
  (CallFunction|DeactiveAIMovement)
  (Collision|SetActorEnableCollision false)
  (bind _asbp_marine (Utilities|Casting|CastToBP_Marine (Game|GetPlayerCharacter 0)))
  (Default|AddEnemyKills _asbp_marine)
  (bind _asbp_mars_marine_game_mode (Utilities|Casting|CastToBP_MarsMarine_GameMode (Game|GetGameMode)))
  (Default|RegisterEnemyDeath _asbp_mars_marine_game_mode self))

(fn IsAlive
  (return (not (Variables|Default|GetIs%20Dead))))

(fn CanAttack
  (return (Math|Boolean|ANDBoolean (CallFunction|IsAlive) (CallFunction|IsWithinAttackRange) (not (CallFunction|IsAttacking)))))