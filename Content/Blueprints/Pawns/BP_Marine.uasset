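; BP_Marine is the player pawn for a twin-stick style shooter, with world-axis movement, a HUD, health and a kill counter.
; Each tick it yaws the control rotation toward thumbstick direction or smoothed mouse velocity, using deadzones and the last key's device type.
; Firing loops a timed hitscan trace from the muzzle socket, applying damage and impact effects alongside muzzle flash and sound.
; Zero health sets IsDead, stopping fire, movement and aiming.
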(event EventBeginPlay
  ;[1 1 1] Create HUD
  (bind _returnvalue (UserInterface|CreateWidget "/Game/UI/WB_PlayerHUD.WB_PlayerHUD_C" 0 self))
  (UserInterface|Viewport|AddtoViewport _returnvalue 0))

(event EventTick
  (params (DeltaSeconds :type Float%20%28single-precision%29))
  ;[1 1 1] Update Player`s Aim
  (CallFunction|UpdateAim))

(event Game|Damage|EventAnyDamage
  (params (Damage :type Float%20%28single-precision%29) (DamageType :type Damage%20Type%20Object%20Reference) (InstigatedBy :type Controller%20Object%20Reference) (DamageCauser :type Actor%20Object%20Reference))
  ;[1 1 1] Take damage
  (bind _health (Properties|DecreaseHealth Damage))
  (if (== _health 0.0)
    (Variables|PlayersProperties|SetIs%20Dead true)
    (Animation|StopFiringWeapon)))

(event Input|ActionEvents|InputActionFireWeapon
  (params (Key :type Key%20Structure))
  ;[1 1 1] Fire weapon
  (:Pressed
    (Animation|StartFiringWeapon))
  (:Released
    (Animation|StopFiringWeapon)))

(event Input|AxisEvents|InputAxisForward/Backward
  (params (AxisValue :type Float%20%28single-precision%29))
  ;[1 1 1] Movement
  (if (Properties|IsAlive)
    (Pawn|Input|AddMovementInput "1.000000, 0, 0" AxisValue false)))

(event Input|AxisEvents|InputAxisLeft/Right
  (params (AxisValue :type Float%20%28single-precision%29))
  ;[1 1 1] Movement
  (if (Properties|IsAlive)
    (Pawn|Input|AddMovementInput "0.000000,1.000000, 0" AxisValue false)))

(event Input|KeyboardEvents|AnyKey
  (params (Key :type Key%20Structure))
  ;[1 1 1] Controller of input type
  (:Pressed
    (Variables|GamePlay|SetIs%20Gamepad%20Active (Class|KismetInputLibrary|KeyIsGamepadKey Key))))

(event Input|KeyboardEvents|Escape
  (params (Key :type Key%20Structure))
  ;[1 1 1] Exit Game
  (:Pressed
    (Game|QuitGame 0 "Quit")))

(fn ConstructionScript)

(fn UpdateAim
  (if (Properties|IsAlive)
    (if (Variables|GamePlay|GetIs%20Gamepad%20Active)
      (ThumbstickAim|UpdateThumbstickAim)
      (else
        (MouseAim|UpdateMouseAim)))))

(fn IsThumbstickAboveDeadzone
  (return (> (Math|Vector2D|Vector2DLength (Math|Vector2D|MakeVector2D (Input|AxisValues|GetThumbstickAimUp) (Input|AxisValues|GetThumbstickAimRight))) (Variables|ThumbstickAim|GetThumbstick%20Deadzone))))

(fn GetMouseVelocity
  (bind _returnvalue (Game|GetPlayerController 0))
  (bind (_deltax _deltay) (Class|PlayerController|GetInputMouseDelta _returnvalue))
  (return (/ (Math|Vector2D|MakeVector2D _deltax _deltay) (Utilities|Time|GetWorldDeltaSeconds))))

(fn IsMouseAboveDeadzone
  (return (> (Math|Vector2D|Vector2DLength (MouseAim|GetMouseVelocity)) (Variables|MouseAim|GetMouse%20Deadzone))))

(fn UpdateMouseAim
  (if (MouseAim|IsMouseAboveDeadzone)
    (Pawn|SetControlRotation (Game|GetPlayerController 0) (MouseAim|GetMouseAimDirection))))

(fn GetMouseAimDirection
  (bind _returnvalue (MouseAim|GetMouseVelocity))
  (return (Math|Interpolation|RInterpTo (Pawn|GetControlRotation (Game|GetPlayerController 0) :!class /Script/Engine.Controller) (Math|Rotator|MakeRotator 0.0 0.0 (Class|KismetMathLibrary|DegAtan2 (.x _returnvalue) (.y _returnvalue))) (Utilities|Time|GetWorldDeltaSeconds) (Variables|MouseAim|GetMouse%20Smoothing%20Strenght))))

(fn UpdateThumbstickAim
  (if (ThumbstickAim|IsThumbstickAboveDeadzone)
    (Pawn|SetControlRotation (Game|GetPlayerController 0) (ThumbstickAim|GetThumbstickAimDirection))))

(fn GetThumbstickAimDirection
  (return (Math|Rotator|MakeRotator 0.0 0.0 (Class|KismetMathLibrary|DegAtan2 (Input|AxisValues|GetThumbstickAimRight) (Input|AxisValues|GetThumbstickAimRight)))))

(fn StartFiringWeapon
  (if (Properties|IsAlive)
    (Components|Activation|Activate (Variables|Default|GetP_AssaultRifle_MF) false)
    (bind _returnvalue (Audio|SpawnSound2D "/Game/Sounds/Weapon_AssaultRifle/Stereo/SC_WeaponFireLoop.SC_WeaponFireLoop" 1.0 1.0 0.0 0))
    (Variables|Default|SetWeapon%20Fire%20Sound _returnvalue)
    (Trace|WeaponTrace)
    (Utilities|Time|SetTimerbyFunctionName 0 "Weapon Trace" (Variables|Weapon|GetWeapon%20Fire%20Rate) true)))

(fn StopFiringWeapon
  (bind _weapon_fire_sound (Variables|Default|GetWeapon%20Fire%20Sound))
  (Components|Activation|Deactivate (Variables|Default|GetP_AssaultRifle_MF))
  (Utilities|IsValid _weapon_fire_sound
    (:Is%20Valid
      (Audio|Components|Audio|Stop _weapon_fire_sound)
      (Utilities|Time|ClearTimerbyFunctionName 0 "Weapon Trace")
      (if (Properties|IsAlive)
        (Audio|SpawnSound2D "/Game/Sounds/Weapon_AssaultRifle/Stereo/SC_WeaponFireEnd.SC_WeaponFireEnd" 1.0 1.0 0.0 0)))))

(fn DecreaseHealth
  (params (Damage :type Float%20%28single-precision%29))
  (bind _output_get (Variables|PlayersProperties|SetHealth (Math|Float|Clamp(Float) (- (Variables|PlayersProperties|GetHealth) Damage) 0.0 1e+02)))
  (return _output_get))

(fn IsAlive
  (return (not (Variables|PlayersProperties|GetIs%20Dead))))

(fn WeaponTrace
  (bind _outhit (Collision|LineTraceByChannel (Trace|GetWeaponTraceStartPoint) (Trace|GetWeaponTraceEndPoint) "TraceTypeQuery1" false 0 "None"))
  (if (.bBlockingHit (Collision|BreakHitResult _outhit))
    (Game|Damage|ApplyDamage (.HitActor (Collision|BreakHitResult _outhit)) (Variables|Weapon|GetWeapon%20Damage) 0 0)
    (CallFunction|SpawnImpactHit (.Location (Collision|BreakHitResult _outhit)))))

(fn GetWeaponTraceStartPoint
  (return (Transformation|GetSocketLocation (Variables|Default|GetWeapon) "MuzzleFlashSocket")))

(fn GetWeaponTraceEndPoint
  (return (+ (Trace|GetWeaponTraceStartPoint) (* (Math|Vector|GetForwardVector (Pawn|GetControlRotation :!class /Script/Engine.Pawn)) (Variables|Weapon|GetWeapon%20Range)))))

(fn AddEnemyKills
  (Math|Integer|IncrementInt (Variables|PlayersProperties|GetEnemy%20Kills)))

(fn SpawnImpactHit
  (params (Hit%20Location :type Vector))
  (Effects|SpawnEmitteratLocation "/Game/Effects/Weapons/Impacts/P_AssaultRifle_IH.P_AssaultRifle_IH" Hit%20Location))

(fn AddHealth
  (params (Health%20to%20add :type Float%20%28single-precision%29))
  (Variables|PlayersProperties|SetHealth (Math|Float|Clamp(Float) (+ (Variables|PlayersProperties|GetHealth) Health%20to%20add) 0.0 1e+02)))

(fn IsHealthFull
  (return (== (Variables|PlayersProperties|GetHealth) 1e+02)))