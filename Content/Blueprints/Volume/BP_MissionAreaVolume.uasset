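; BP_MissionAreaVolume is a volume that punishes the player for leaving the mission area.
; When a BP_Marine ends overlap, it sets that marine's outside-area flag and starts a looping Kill Player timer paced by TimerToPlayerTakeDamage.
; Each tick of that timer applies fixed damage to player character 0, regardless of which marine left.
; Re-entering clears both the flag and the timer.
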(event EventBeginPlay)

(event EventTick
  (params (DeltaSeconds :type Float%20%28single-precision%29)))

(event Collision|EventActorBeginOverlap
  (params (OtherActor :type Actor%20Object%20Reference))
  ;[1 1 1] Marine enters mission area
  (bind _asbp_marine (Utilities|Casting|CastToBP_Marine OtherActor))
  (Variables|/Game/Blueprints/Pawns/BP_Marine.BP_Marine_C|SetIs%20Player%20Outside%20Mission%20Area _asbp_marine false)
  (Utilities|Time|ClearTimerbyFunctionName 0 "Kill Player"))

(event Collision|EventActorEndOverlap
  (params (OtherActor :type Actor%20Object%20Reference))
  ;[1 1 1] Marine leaves mission area
  (bind _asbp_marine (Utilities|Casting|CastToBP_Marine OtherActor))
  (Variables|/Game/Blueprints/Pawns/BP_Marine.BP_Marine_C|SetIs%20Player%20Outside%20Mission%20Area _asbp_marine true)
  (Utilities|Time|SetTimerbyFunctionName 0 "Kill Player" (Variables|Default|GetTimer%20To%20Player%20Take%20Damage) true))

(fn ConstructionScript)

(fn KillPlayer
  (Game|Damage|ApplyDamage (Game|GetPlayerCharacter 0) 15.0 0 0))